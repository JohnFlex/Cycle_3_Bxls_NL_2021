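; BP_CPawn is a pawn Blueprint that moves along the player controller's forward vector from the "forward" axis input.
; It also holds two counter helpers on the Inc variable: a function that increments and prints it, and a macro that increments it and then waits on a Delay.
; Neither helper is called in the event graph, and BeginPlay, overlap and Tick are empty.
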(event `self.ReceiveBeginPlay`)

(event `self.ReceiveTick`
  (params (DeltaSeconds :type "Float (single-precision)")))

(event `InputAxis|forward`
  (params (AxisValue :type "Float (single-precision)"))
  (`self.AddMovementInput` (`self.GetActorForwardVector` (`GameplayStatics.GetPlayerController` 0)) AxisValue))

(fn `Fct_Increment`
  (bind _output_get (set `self.inc` (+ (`self.inc`) 1)))
  (`KismetSystemLibrary.PrintString` (`KismetStringLibrary.Conv_IntToString` _output_get)))

(fn `UserConstructionScript`)